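; Bullet projectile that flies forward and destroys actors tagged Enemy.
; On spawn it plays audio, creates its own WB_Hub widget, increments that widget's shot counter (Disparos) and passes it to UpdateWidget.
; Each tick sets the mesh's relative location from forward vector, Speed and an incrementing counter, so movement is frame-rate dependent.
; A capsule overlap with an enemy spawns a Niagara explosion there and destroys both actors.
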(event OnComponentBeginOverlap(Capsule)
  (params (OverlappedComponent :type Primitive%20Component%20Object%20Reference) (OtherActor :type Actor%20Object%20Reference) (OtherComp :type Primitive%20Component%20Object%20Reference) (OtherBodyIndex :type Integer) (bFromSweep :type Boolean) (SweepResult :type Hit%20Result%20Structure%20%28by%20ref%29))
  (if (Actor|ActorHasTag OtherActor "Enemy")
    (Utilities|FlowControl|DoOnce false
      (:Completed
        (CallFunction|Explosion (Transformation|GetActorTransform OtherActor))
        (Actor|DestroyActor OtherActor)))))

(event Custom|Explosion
  (params (ubicacion :type Transform))
  (Niagara|SpawnSystematLocation "/Game/vfx/Niagara_Explosion_03.Niagara_Explosion_03" (.location ubicacion) (.rotation ubicacion) (.scale ubicacion) true true "AutoRelease")
  (Actor|DestroyActor))

(event EventBeginPlay
  (Variables|Default|SetPlayer (Game|GetPlayerCharacter 0))
  (Audio|Components|Audio|Play (Variables|Default|GetAudio) 0.0)
  ;[0.15 0.01484 0.01484 0.5] mmm
  (bind _returnvalue (UserInterface|CreateWidget "/Game/blueprints/UI/WB_Hub.WB_Hub_C" (Game|GetPlayerController 0)))
  (bind _output_get (Variables|Default|SetHud _returnvalue))
  (bind _result (Math|Integer|IncrementInt (Variables|/Game/blueprints/UI/WB_Hub.WB_Hub_C|GetDisparos _output_get))
    (:%20%20
      (Default|UpdateWidget _output_get 0 _result 0 0.0 false))))

(event EventTick
  (params (DeltaSeconds :type Float%20%28single-precision%29))
  ;[0.15 0.15 0.15 0.5] Avance
  (bind _result (Math|Float|IncrementFloat (Variables|Default|GetposicionInicial))
    (:%20%20
      (Transformation|SetRelativeLocation (Variables|Default|GetStaticMesh) (* (Transformation|GetActorForwardVector) (* _result (Variables|Default|GetSpeed))) false false))))

(fn ConstructionScript)