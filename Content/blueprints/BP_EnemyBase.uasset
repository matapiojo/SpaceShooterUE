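; BP_EnemyBase is an enemy ship that moves along world X and damages the player on contact.
; BeginPlay randomizes mesh and speed, then derives box extent and spotlight offset from mesh bounds, though each random lookup is separate.
; Tick adds forward X times Speed plus DeltaSeconds, so movement is frame-rate dependent.
; The Box's first overlap with a Player-tagged actor calls DamageActor on the cached MyCharacter.
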(event OnComponentBeginOverlap(Box)
  (params (OverlappedComponent :type Primitive%20Component%20Object%20Reference) (OtherActor :type Actor%20Object%20Reference) (OtherComp :type Primitive%20Component%20Object%20Reference) (OtherBodyIndex :type Integer) (bFromSweep :type Boolean) (SweepResult :type Hit%20Result%20Structure%20%28by%20ref%29))
  (if (Actor|ActorHasTag OtherActor "Player")
    (Utilities|FlowControl|DoOnce false
      (:Completed
        (Default|DamageActor (Variables|Default|GetAs%20My%20Character))))))

(event EventBeginPlay
  (bind _todasnaves (Variables|Default|GetTodasNaves))
  (bind _returnvalue (Utilities|Array|Length _todasnaves))
  (bind _returnvalue_2 (- _returnvalue 1))
  (bind _returnvalue_3 (Math|Random|RandomIntegerinRange 0 _returnvalue_2))
  (bind _output (Utilities|Array|Get(acopy) _todasnaves _returnvalue_3))
  (bind _returnvalue_4 (StaticMesh|GetBoundingBox _output))
  (bind _asmy_character (Utilities|Casting|CastToMyCharacter (Game|GetPlayerCharacter 0)))
  (Variables|Default|SetAs%20My%20Character _asmy_character)
  (Components|StaticMesh|SetStaticMesh (Variables|Default|GetStaticMesh) _output)
  (Components|Box|SetBoxExtent (Variables|Default|GetBox) (Math|Vector|MakeVector (- (.x (.max _returnvalue_4)) (.x (.min _returnvalue_4))) (- (.y (.max _returnvalue_4)) (.y (.min _returnvalue_4))) (- (.z (.max _returnvalue_4)) (.z (.min _returnvalue_4)))) true)
  (Variables|Default|Setspeed (Math|Random|RandomFloatinRange (- (Variables|Default|Getspeed) 5.0) (Variables|Default|Getspeed)))
  (Transformation|AddLocalOffset (Variables|Default|GetSpotLight) (Math|Vector|MakeVector (.x (.max _returnvalue_4)) 0.0 0.0) false false)
  (Collision|SetCollisionEnabled (Variables|Default|GetStaticMesh) "NoCollision"))

(event EventTick
  (params (DeltaSeconds :type Float%20%28single-precision%29))
  (Transformation|AddWorldOffset (Variables|Default|GetScene) (Math|Vector|MakeVector (+ DeltaSeconds (* (.x (Transformation|GetActorForwardVector)) (Variables|Default|Getspeed))) 0.0 0.0) false false))

(fn ConstructionScript)