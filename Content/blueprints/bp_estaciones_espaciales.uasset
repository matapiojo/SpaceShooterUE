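; Space station actor that serves as a non-colliding moving prop, drifting along world X.
; On BeginPlay it tilts and scales its static mesh, offsets it locally by the player character's location plus an X offset, then shows it with collision disabled.
; Each Tick shifts the mesh along negative X by forward-vector X times Speed plus DeltaSeconds, so movement depends on frame rate because delta time is added, not multiplied.
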(event EventBeginPlay
  (bind _staticmesh (Variables|Default|GetStaticMesh))
  (bind _staticmesh_2 (Variables|Default|GetStaticMesh))
  (Transformation|SetRelativeRotation _staticmesh "0.000000,45.000000,45.000000" false false)
  (Transformation|SetRelativeScale3D _staticmesh (Math|Conversions|ToVector(Float) (Variables|Default|GetescalaEstacion)))
  (Transformation|AddLocalOffset _staticmesh (+ (Transformation|GetActorLocation (Game|GetPlayerCharacter 0)) (Math|Vector|MakeVector (Math|Conversions|ToFloat(Integer) (Variables|Default|Getoffset)) 0.0 0.0)) false false)
  (Rendering|SetVisibility _staticmesh_2 true false)
  (Collision|SetCollisionEnabled _staticmesh_2 "NoCollision"))

(event EventTick
  (params (DeltaSeconds :type Float%20%28single-precision%29))
  (Transformation|AddWorldOffset (Variables|Default|GetStaticMesh) (Math|Vector|MakeVector (* (+ DeltaSeconds (* (.x (Transformation|GetActorForwardVector)) (Variables|Default|Getspeed))) -1.0) 0.0 0.0) false false))

(fn ConstructionScript)