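; Player spaceship character that moves on world axes, fires, raises a shield and tracks lives.
; Enhanced Input drives movement with Timeline-based banking, alternating shots from two fire points with a missile counter, and a shield active until input completes.
; BeginPlay caches the game mode and creates the HUD widget, which DamageActor updates with remaining lives except when they reach zero.
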(event Custom|DamageActor
  (bind _output_get (Variables|Default|SetVidas (- (Variables|Default|GetVidas) 1)))
  (if (not (== _output_get 0))
    (Default|UpdateWidget (Variables|Default|GetHud) 0 0 _output_get 0.0 false)))

(event Input|EnhancedActionEvents|EnhancedInputActionAI_disparo
  (params (ActionValue :type Boolean) (ElapsedSeconds :type Float%20%28double-precision%29) (TriggeredSeconds :type Float%20%28double-precision%29) (InputAction :type Input%20Action%20Object%20Reference :default "/Game/blueprints/Input/AI_disparo.AI_disparo"))
  (bind _ammo (Variables|Default|GetAmmo))
  (:Started
    (Utilities|FlowControl|FlipFlop
      (:A
        (Game|SpawnActorfromClass _ammo (Math|Transform|MakeTransform (Transformation|GetWorldLocation (Variables|Default|GetFirePointDer)) "0, 0, 0" "1.000000,1.000000,1.000000") "Undefined" "MultiplyWithRoot" 0 0))
      (:B
        (Game|SpawnActorfromClass _ammo (Math|Transform|MakeTransform (Transformation|GetWorldLocation (Variables|Default|GetFirePointIzq)) "0, 0, 0" "1.000000,1.000000,1.000000") "Undefined" "MultiplyWithRoot" 0 0)))
    (bind _result (Math|Integer|IncrementInt (Variables|Default|GetCantMisiles))
      (:%20%20
        (Variables|Default|SetCantMisiles _result)))))

(event Input|EnhancedActionEvents|EnhancedInputActionAI_Mover
  (params (ActionValue :type Vector%202D%20Structure) (ElapsedSeconds :type Float%20%28double-precision%29) (TriggeredSeconds :type Float%20%28double-precision%29) (InputAction :type Input%20Action%20Object%20Reference :default "/Game/blueprints/Input/AI_Mover.AI_Mover"))
  (Variables|Default|SetAction%20Value%20X (.x ActionValue))
  (Pawn|Input|AddMovementInput (Math|Vector|GetRightVector "0, 0, 0") (.x ActionValue) false)
  (Pawn|Input|AddMovementInput (Math|Vector|GetForwardVector "0, 0, 0") (.y ActionValue) false)
  (bind _newtrack_0 (Timeline|Timeline Play)
    (:Update
      (Transformation|SetWorldRotation (Variables|Default|GetSpaceShip) (Math|Rotator|MakeRotator (* -1.0 (* (* _newtrack_0 (Variables|Default|GetanguloDoblar)) (Variables|Default|GetAction%20Value%20X))) 0.0 (+ (* (* _newtrack_0 (Variables|Default|GetanguloDoblar)) (Variables|Default|GetAction%20Value%20X)) 1.8e+02)) false false)
      (Timeline|Timeline Reverse))))

(event Input|EnhancedActionEvents|EnhancedInputActionAI_Shield
  (params (ActionValue :type Boolean) (ElapsedSeconds :type Float%20%28double-precision%29) (TriggeredSeconds :type Float%20%28double-precision%29) (InputAction :type Input%20Action%20Object%20Reference :default "/Game/blueprints/Input/AI_Shield.AI_Shield"))
  (:Started
    (Rendering|SetVisibility (Variables|Default|Getshield) true false)
    (Collision|SetCollisionEnabled (Variables|Default|GetSphere) "QueryOnly")
    (Utilities|FlowControl|Delay 3.0))
  (:Completed
    (Rendering|SetVisibility (Variables|Default|Getshield) false false)
    (Collision|SetCollisionEnabled (Variables|Default|GetSphere) "NoCollision")))

(event EventBeginPlay
  (bind _asplayer_controller (Utilities|Casting|CastToPlayerController (Pawn|GetController)))
  (Utilities|IsValid (PlayerController|LocalPlayerSubsystems|GetEnhancedInputLocalPlayerSubsystem _asplayer_controller)
    (:Is%20Valid
      (Input|AddMappingContext (PlayerController|LocalPlayerSubsystems|GetEnhancedInputLocalPlayerSubsystem _asplayer_controller) "/Game/blueprints/Input/IMC_Input.IMC_Input" 0 "(bIgnoreAllPressedKeysUntilRelease=True,bForceImmediately=False,bNotifyUserSettings=False)")
      (bind _asmy_game_mode (Utilities|Casting|CastToMyGameMode (Game|GetGameMode)))
      (Variables|Default|SetAs%20My%20Game%20Mode _asmy_game_mode)
      (Collision|SetCollisionEnabled (Variables|Default|GetSphere) "NoCollision")
      (bind _returnvalue (UserInterface|CreateWidget "/Game/blueprints/UI/WB_Hub.WB_Hub_C" (Game|GetPlayerController 0)))
      (Variables|Default|SetHud _returnvalue))))

(fn ConstructionScript)