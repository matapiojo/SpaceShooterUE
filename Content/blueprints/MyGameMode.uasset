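; MyGameMode is a game mode Blueprint that tracks a progress value and relays player death to the HUD.
; On BeginPlay it casts the first player controller's HUD to BP_SpaceS_HUD and caches it.
; Tick adds IncrementTick to Progreso every frame without delta-time scaling, so progress depends on frame rate.
; The PlayerDead event calls PlayerKill on the cached HUD.
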(event Custom|PlayerDead
  (Default|PlayerKill (Variables|Default|GetHUD%20Player)))

(event EventBeginPlay
  (bind _asbp_space_s_hud (Utilities|Casting|CastToBP_SpaceS_HUD (HUD|GetHUD (Game|GetPlayerController 0))))
  (Variables|Default|SetHUD%20Player _asbp_space_s_hud))

(event EventTick
  (params (DeltaSeconds :type Float%20%28single-precision%29))
  (Variables|Default|SetProgreso (+ (Variables|Default|GetIncrementTick) (Variables|Default|GetProgreso))))

(fn ConstructionScript)