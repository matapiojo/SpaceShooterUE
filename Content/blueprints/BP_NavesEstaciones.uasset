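; BP_NavesEstaciones is a spawner that keeps creating Enemy actors, apparently ships, near the player's lane.
; Tick feeds a random Delay of a few seconds into CrearNave, so the latent node acts as a repeating timer.
; Each spawn takes a random absolute world X, a random Y offset around the player, the player's Z and scale, and a fixed half-turn rotation.
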(event Custom|Crear%20Nave
  (bind _returnvalue (Game|GetPlayerCharacter 0))
  (bind _returnvalue_2 (Transformation|GetActorTransform _returnvalue))
  (Game|SpawnActorfromClass (Variables|Default|GetEnemy) (Math|Transform|MakeTransform (Math|Vector|MakeVector (Math|Random|RandomFloatinRange 1.5e+03 2e+03) (+ (Math|Random|RandomFloatinRange -3.5e+02 3.5e+02) (.y (.location _returnvalue_2))) (.z (.location _returnvalue_2))) "0.000000,180.000000,0.000000" (.scale _returnvalue_2)) "Undefined" "MultiplyWithRoot" 0 0))

(event EventTick
  (params (DeltaSeconds :type Float%20%28single-precision%29))
  (Utilities|FlowControl|Delay (Math|Random|RandomFloatinRange 2.0 5.0))
  (CallFunction|CrearNave))

(fn ConstructionScript)