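; Non-colliding ship actor that endlessly flies its mesh between two markers, A and B, placed around the player.
; Each pass, ABLocation re-places both markers at random heights and player-relative Y offsets, negating their X on alternate calls via a FlipFlop.
; FireShip activates Niagara, snaps the mesh to A, moves it to B over a random duration using a yaw-negated look-at rotation, then deactivates Niagara and calls itself again.
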(event Custom|FireShip
  (bind _a (Variables|Default|GetA))
  (bind _staticmesh (Variables|Default|GetStaticMesh))
  (bind _b (Variables|Default|GetB))
  (bind _returnvalue (Transformation|GetWorldLocation _b))
  (bind _returnvalue_2 (Transformation|GetWorldLocation _a))
  (bind _returnvalue_3 (Math|Rotator|FindLookatRotation _returnvalue_2 _returnvalue))
  (Components|Activation|SetActive (Variables|Default|GetNiagara) true false)
  (Collision|SetCollisionEnabled (Variables|Default|GetStaticMesh) "NoCollision")
  (CallFunction|ABLocation)
  (Transformation|SetWorldLocation _staticmesh _returnvalue_2 false false)
  (Components|MoveComponentTo _staticmesh _returnvalue (Math|Rotator|MakeRotator (.roll _returnvalue_3) (.pitch _returnvalue_3) (* (.yaw _returnvalue_3) -1.0)) false false (Math|Random|RandomFloatinRange 0.2 3.0) false)
  (Components|Activation|SetActive (Variables|Default|GetNiagara) false true)
  (CallFunction|FireShip))

(event EventBeginPlay
  (CallFunction|FireShip))

(fn ConstructionScript)

(fn ABLocation
  (bind _returnvalue (Game|GetPlayerCharacter 0))
  (Utilities|FlowControl|FlipFlop
    (:A
      (Variables|Default|Setdireccion 1.0))
    (:B
      (Variables|Default|Setdireccion -1.0)))
  (Transformation|SetWorldLocation (Variables|Default|GetA) (Math|Vector|MakeVector (* (.x (Transformation|GetWorldLocation (Variables|Default|GetA))) (Variables|Default|Getdireccion)) (.y (- (Transformation|GetActorLocation _returnvalue) (Math|Vector|MakeVector (Math|Random|RandomFloatinRange 5e+02 1.2e+03) (Math|Random|RandomFloatinRange 1.5e+03 3e+03) 0.0))) (Math|Random|RandomFloatinRange -1e+03 1e+03)) false false)
  (Transformation|SetWorldLocation (Variables|Default|GetB) (Math|Vector|MakeVector (* (.x (Transformation|GetWorldLocation (Variables|Default|GetB))) (Variables|Default|Getdireccion)) (.y (+ (Transformation|GetActorLocation _returnvalue) (Math|Vector|MakeVector (Math|Random|RandomFloatinRange 5e+02 1.2e+03) (Math|Random|RandomFloatinRange 1.5e+03 5e+03) 0.0))) (Math|Random|RandomFloatinRange -1e+03 1e+03)) false false))